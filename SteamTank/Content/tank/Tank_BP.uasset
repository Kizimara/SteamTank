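; Player-controllable tank Blueprint that wires its mesh parts to aiming and movement components and handles input.
; On BeginPlay it hands the barrel and turret to TankAiming and both tracks to TankMovement, assigning their static meshes.
; Aim axes rotate an azimuth gimbal for yaw and a spring arm for pitch, drive axes send movement intents to TankMovement, and the Fire action calls Fire.
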(event EventBeginPlay
  (Utilities|FlowControl|Sequence
    (:then_0
      (Class|TankAimingComponent|Initialise (Variables|Default|GetTankAiming) (Variables|Default|GetTankBarrel) (Variables|Default|GetTurret))
      (Components|StaticMesh|SetStaticMesh (Variables|Default|GetTankBarrel) "/Game/tank/tank_fbx_Barrel.tank_fbx_Barrel")
      (Components|StaticMesh|SetStaticMesh (Variables|Default|GetTurret) "/Game/tank/tank_fbx_Turret.tank_fbx_Turret"))
    (:then_1
      (Class|TankMovementComponent|Initialise (Variables|Default|GetTankMovement) (Variables|Default|GetLeftTrack) (Variables|Default|GetRightTrack))
      (Components|StaticMesh|SetStaticMesh (Variables|Default|GetLeftTrack) "/Game/tank/tank_fbx_Track_track_001.tank_fbx_Track_track_001")
      (Components|StaticMesh|SetStaticMesh (Variables|Default|GetRightTrack) "/Game/tank/tank_fbx_Track_track_001.tank_fbx_Track_track_001"))))

(event Input|ActionEvents|InputActionFire
  (params (Key :type Key%20Structure))
  (:Pressed
    (Class|Tank|Fire)))

(event Input|AxisEvents|InputAxisAimAzimut
  (params (AxisValue :type Float%20%28single-precision%29))
  ;[1 1 1] Aiming input binding
  (Transformation|AddLocalRotation (Variables|Default|GetAzimutGimble) (Math|Rotator|MakeRotator 0.0 0.0 (* AxisValue 3.0)) false false))

(event Input|AxisEvents|InputAxisAimAltttude
  (params (AxisValue :type Float%20%28single-precision%29))
  ;[1 1 1] Aiming input binding
  (Transformation|AddLocalRotation (Variables|Default|GetSpringArm) (Math|Rotator|MakeRotator 0.0 (* AxisValue 3.0) 0.0) false false))

(event Input|AxisEvents|InputAxisTurn
  (params (AxisValue :type Float%20%28single-precision%29))
  (Class|TankMovementComponent|IntendTurnRight (Variables|Default|GetTankMovement) AxisValue))

(event Input|AxisEvents|InputAxisMoveForward
  (params (AxisValue :type Float%20%28single-precision%29))
  (Class|TankMovementComponent|IntendMoveForward (Variables|Default|GetTankMovement) AxisValue))

(fn ConstructionScript)